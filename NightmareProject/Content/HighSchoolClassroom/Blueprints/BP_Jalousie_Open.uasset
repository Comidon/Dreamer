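; BP_Jalousie_Open is a window blind prop for the high school classroom whose slats share one adjustable tilt.
; The construction script applies the RotJalousie variable as the relative rotation of 28 individual static mesh components, so they all tilt together when the actor is constructed.
; The script contains no runtime logic or animation.
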(fn `UserConstructionScript`
  ;[1 1 1] Rotation Jalousie
  (`SceneComponent.K2_SetRelativeRotation` (`self.StaticMesh6`) (`self.RotJalousie`) false false)
  (`SceneComponent.K2_SetRelativeRotation` (`self.StaticMesh2`) (`self.RotJalousie`) false false)
  (`SceneComponent.K2_SetRelativeRotation` (`self.StaticMesh3`) (`self.RotJalousie`) false false)
  (`SceneComponent.K2_SetRelativeRotation` (`self.StaticMesh4`) (`self.RotJalousie`) false false)
  (`SceneComponent.K2_SetRelativeRotation` (`self.StaticMesh5`) (`self.RotJalousie`) false false)
  (`SceneComponent.K2_SetRelativeRotation` (`self.StaticMesh1`) (`self.RotJalousie`) false false)
  (`SceneComponent.K2_SetRelativeRotation` (`self.StaticMesh7`) (`self.RotJalousie`) false false)
  (`SceneComponent.K2_SetRelativeRotation` (`self.StaticMesh8`) (`self.RotJalousie`) false false)
  (`SceneComponent.K2_SetRelativeRotation` (`self.StaticMesh9`) (`self.RotJalousie`) false false)
  (`SceneComponent.K2_SetRelativeRotation` (`self.StaticMesh10`) (`self.RotJalousie`) false false)
  (`SceneComponent.K2_SetRelativeRotation` (`self.StaticMesh11`) (`self.RotJalousie`) false false)
  (`SceneComponent.K2_SetRelativeRotation` (`self.StaticMesh12`) (`self.RotJalousie`) false false)
  (`SceneComponent.K2_SetRelativeRotation` (`self.StaticMesh14`) (`self.RotJalousie`) false false)
  (`SceneComponent.K2_SetRelativeRotation` (`self.StaticMesh15`) (`self.RotJalousie`) false false)
  (`SceneComponent.K2_SetRelativeRotation` (`self.StaticMesh16`) (`self.RotJalousie`) false false)
  (`SceneComponent.K2_SetRelativeRotation` (`self.StaticMesh13`) (`self.RotJalousie`) false false)
  (`SceneComponent.K2_SetRelativeRotation` (`self.StaticMesh17`) (`self.RotJalousie`) false false)
  (`SceneComponent.K2_SetRelativeRotation` (`self.StaticMesh18`) (`self.RotJalousie`) false false)
  (`SceneComponent.K2_SetRelativeRotation` (`self.StaticMesh19`) (`self.RotJalousie`) false false)
  (`SceneComponent.K2_SetRelativeRotation` (`self.StaticMesh20`) (`self.RotJalousie`) false false)
  (`SceneComponent.K2_SetRelativeRotation` (`self.StaticMesh21`) (`self.RotJalousie`) false false)
  (`SceneComponent.K2_SetRelativeRotation` (`self.StaticMesh22`) (`self.RotJalousie`) false false)
  (`SceneComponent.K2_SetRelativeRotation` (`self.StaticMesh23`) (`self.RotJalousie`) false false)
  (`SceneComponent.K2_SetRelativeRotation` (`self.StaticMesh24`) (`self.RotJalousie`) false false)
  (`SceneComponent.K2_SetRelativeRotation` (`self.StaticMesh25`) (`self.RotJalousie`) false false)
  (`SceneComponent.K2_SetRelativeRotation` (`self.StaticMesh26`) (`self.RotJalousie`) false false)
  (`SceneComponent.K2_SetRelativeRotation` (`self.StaticMesh27`) (`self.RotJalousie`) false false)
  (`SceneComponent.K2_SetRelativeRotation` (`self.StaticMesh28`) (`self.RotJalousie`) false false))