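; BP_Clock is an animated clock prop for the high school classroom, with moving second, minute and hour hands.
; On BeginPlay it starts three separate timelines, one per hand, each driving that arrow component's relative pitch from its rotation track.
; Hand motion comes entirely from the timeline curves, with no system time lookup or initial time setup.
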(event `self.ReceiveBeginPlay`
  (`|ExecutionSequence`
    (:`then_0`
      (bind (_direction _secondrot) (`Timeline|SecondAnim`)
        (:`Update`
          (`SceneComponent.K2_SetRelativeRotation` (`self.Arrow_Second`) (`KismetMathLibrary.MakeRotator` 0.0 _secondrot) false false))))
    (:`then_1`
      (bind (_direction_2 _minuterot) (`Timeline|MinuteAnim`)
        (:`Update`
          (`SceneComponent.K2_SetRelativeRotation` (`self.Arrow_Minute`) (`KismetMathLibrary.MakeRotator` 0.0 _minuterot) false false))))
    (:`then_2`
      (bind (_direction_3 _hourrot) (`Timeline|HourAnim`)
        (:`Update`
          (`SceneComponent.K2_SetRelativeRotation` (`self.Arrow_Hour`) (`KismetMathLibrary.MakeRotator` 0.0 _hourrot) false false))))))

(fn `UserConstructionScript`)