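; BP_Door is a configurable classroom door prop built from frame, door and handle components.
; Its construction script applies materials chosen by index from separate lists to specific slots on the frame and door.
; It also sets the relative rotations of door and handle from variables, attaching the handle to the door so it follows the swing.
; The graph contains only this setup, with no runtime open or close logic.
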(fn `UserConstructionScript`
  (bind _door (`self.Door`))
  (bind _doorframe (`self.DoorFrame`))
  (bind _door_2 (`self.Door`))
  (bind _item (`KismetArrayLibrary.Array_Get` (`self.List material for DoorFrame`) (`self.Choose material for DoorFrame`)))
  (bind _item_2 (`KismetArrayLibrary.Array_Get` (`self.List material for Door`) (`self.Choose material for Door`)))
  (`|ExecutionSequence`
    (:`then_0`
      ;[1 1 1] Choose material for DoorFrame
      (`PrimitiveComponent.SetMaterial` _doorframe 0 _item)
      (`PrimitiveComponent.SetMaterial` _doorframe 2 _item))
    (:`then_1`
      ;[1 1 1] Choose material for Door
      (`PrimitiveComponent.SetMaterial` _door 1 _item_2)
      (`PrimitiveComponent.SetMaterial` _door 4 _item_2)
      (`PrimitiveComponent.SetMaterial` _door 7 _item_2))
    (:`then_2`
      ;[1 1 1] Rotation Door
      (`SceneComponent.K2_SetRelativeRotation` _door_2 (`self.RotDoor`) false false)
      ;[1 1 1] Attach to Doorhandle
      (`SceneComponent.K2_AttachToComponent` (`self.DoorHandle`) _door_2 "None" "KeepRelative" "KeepRelative" "KeepRelative" true))
    (:`then_3`
      ;[1 1 1] Rotation Handle
      (`SceneComponent.K2_SetRelativeRotation` (`self.DoorHandle`) (`self.RotDoorhandle`) false false))))