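; BP_ChairSchool is a school chair prop for a high school classroom with selectable plastic and metal materials.
; Its construction script picks one entry from each of two material lists using an index variable.
; The plastic choice is applied to the even material slots of the ChairSchool component and the metal choice to the odd slots, so variants update when the actor is constructed.
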(fn `UserConstructionScript`
  (bind _chair_school (`self.Chair_School`))
  (bind _chair_school_2 (`self.Chair_School`))
  (bind _item (`KismetArrayLibrary.Array_Get` (`self.List material for Metal`) (`self.Choose material for Metal`)))
  (bind _item_2 (`KismetArrayLibrary.Array_Get` (`self.List material for Plastic`) (`self.Choose material for Plastic`)))
  (`|ExecutionSequence`
    (:`then_0`
      ;[1 1 1] Choose material for Plastic
      (`PrimitiveComponent.SetMaterial` _chair_school_2 0 _item_2)
      (`PrimitiveComponent.SetMaterial` _chair_school_2 2 _item_2)
      (`PrimitiveComponent.SetMaterial` _chair_school_2 4 _item_2))
    (:`then_1`
      ;[1 1 1] Choose material for Metal
      (`PrimitiveComponent.SetMaterial` _chair_school 1 _item)
      (`PrimitiveComponent.SetMaterial` _chair_school 3 _item)
      (`PrimitiveComponent.SetMaterial` _chair_school 5 _item))))